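; BP_2DTryPlayerController is a player controller that toggles a custom key-mapping menu with the Tab key.
; A FlipFlop alternates between creating a fresh key menu widget with mouse cursor and Game and UI input, and removing it to restore game-only input with the cursor hidden.
; BeginPlay, Tick and the construction script are empty.
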(event EventBeginPlay)

(event EventTick
  (params (DeltaSeconds :type Float%20%28single-precision%29)))

(event Input|KeyboardEvents|Tab
  (params (Key :type Key%20Structure :default "None"))
  (:Pressed
    (Utilities|FlowControl|FlipFlop
      (:A
        (bind _returnvalue (UserInterface|CreateWidget "/Game/blueprint/UI/BP_uiCustomKeyMenu.BP_uiCustomKeyMenu_C"))
        (UserInterface|Viewport|AddtoViewport _returnvalue 0)
        (bind _output_get (Variables|Default|SetkeyMapMenu _returnvalue))
        (Variables|Default|SetbShowMouseCursor true)
        (Input|SetInputModeGameandUI self _output_get "DoNotLock" true))
      (:B
        (Widget|RemovefromParent (Variables|Default|GetkeyMapMenu))
        (Variables|Default|SetbShowMouseCursor false)
        (Input|SetInputModeGameOnly self)))))

(fn ConstructionScript)