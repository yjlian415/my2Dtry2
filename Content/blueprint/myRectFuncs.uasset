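; Function library for a custom MyRect struct, providing 2D rectangle math on the X/Z plane with Top above Bottom.
; It computes size, offsets by a vector, finds how far one rect overhangs another, and shifts a rect in X by reference.
; MyRectAnd combines horizontal overlap with the vertical outer extents, returning a default rect on failed checks.
; MyRectEmpty, despite its name, returns true when either dimension is positive.
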(fn MyRectWidth
  (params (myRect :type My%20Rect%20Structure))
  (bind (_left _top _right) (Utilities|Struct|BreakmyRect myRect))
  (return (- _right _left)))

(fn MyRectHeight
  (params (myRect :type My%20Rect%20Structure))
  (bind (_left _top _right _bottom) (Utilities|Struct|BreakmyRect myRect))
  (return (- _top _bottom)))

(fn MyRectSub
  (params (myRect :type My%20Rect%20Structure) (subRect :type My%20Rect%20Structure))
  (bind (_left _top _right _bottom) (Utilities|Struct|BreakmyRect myRect))
  (bind (_left_2 _top_2 _right_2 _bottom_2) (Utilities|Struct|BreakmyRect subRect))
  (bind _returnvalue (- _left _left_2))
  (bind _returnvalue_2 (- _right _right_2))
  (bind _returnvalue_3 (- _top _top_2))
  (bind _returnvalue_4 (- _bottom _bottom_2))
  (Utilities|FlowControl|Sequence
    (:then_0
      (if (< _returnvalue 0.0)
        (LocalVariables|SetdeltaX _returnvalue)
        (elif (> _returnvalue_2 0.0)
          (LocalVariables|SetdeltaX _returnvalue_2))))
    (:then_1
      (if (> _returnvalue_3 0.0)
        (LocalVariables|SetdeltaY _returnvalue_3)
        (elif (< _returnvalue_4 0.0)
          (LocalVariables|SetdeltaY _returnvalue_4))))
    (:then_2
      (return (Math|Vector|MakeVector (LocalVariables|GetdeltaX) 0.0 (LocalVariables|GetdeltaY))))))

(fn MyRectand
  (params (rectA :type My%20Rect%20Structure) (rectB :type My%20Rect%20Structure))
  (bind (_left _top _right _bottom) (Utilities|Struct|BreakmyRect rectA))
  (bind (_left_2 _top_2 _right_2 _bottom_2) (Utilities|Struct|BreakmyRect rectB))
  (bind _returnvalue (Math|Float|Max(Float) _left _left_2))
  (bind _returnvalue_2 (Math|Float|Max(Float) _top _top_2))
  (bind _returnvalue_3 (Math|Float|Min(Float) _right _right_2))
  (bind _returnvalue_4 (Math|Float|Min(Float) _bottom _bottom_2))
  (if (or (> _returnvalue _returnvalue_3) (< _returnvalue_2 _returnvalue_4))
    (return (Utilities|Struct|MakemyRect 0.0 0.0 0.0 0.0))
    (else
      (return (Utilities|Struct|MakemyRect _returnvalue _returnvalue_2 _returnvalue_3 _returnvalue_4)))))

(fn MyRectAddVector
  (params (myRect :type My%20Rect%20Structure) (vecAdd :type Vector))
  (bind (_left _top _right _bottom) (Utilities|Struct|BreakmyRect myRect))
  (bind (_x _y _z) (Math|Vector|BreakVector vecAdd))
  (return (Utilities|Struct|MakemyRect (+ _left _x) (+ _top _z) (+ _right _x) (+ _bottom _z))))

(fn MyRectEmpty
  (params (myRect :type My%20Rect%20Structure))
  (return (or (> (CallFunction|MyRectWidth myRect) 0.0) (> (CallFunction|MyRectHeight myRect) 0.0))))

(fn MyRectFlitX
  (params (mrRect :type My%20Rect%20Structure%20%28by%20ref%29))
  (bind _output_get (LocalVariables|SettempRect mrRect))
  (bind _result (Math|Float|NegateFloat (+ (.left (Utilities|Struct|BreakmyRect _output_get)) (.right (Utilities|Struct|BreakmyRect _output_get))))
    (:%20%20
      (|SetBy-RefVar mrRect (CallFunction|MyRectAddVector mrRect (Math|Vector|MakeVector _result 0.0 0.0)))
      (return ""))))