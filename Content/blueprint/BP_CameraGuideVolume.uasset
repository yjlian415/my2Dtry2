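; BP_CameraGuideVolume is a box volume that gathers camera guide anchor components and supplies a combined focus location from them.
; It fills FocusAnchors with a component overlap query at BeginPlay, then updates the collection on box begin and end overlaps.
; GetFocusLocation returns the anchors' average world position, weighted by each FocusWeight.
; InitEmpty zeroes the box and disables its overlap events, while AddGuideRefrence allows anchors to be registered directly.
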(event OnComponentBeginOverlap(Box)
  (params (OverlappedComponent :type Primitive%20Component%20Object%20Reference) (OtherActor :type Actor%20Object%20Reference) (OtherComp :type Primitive%20Component%20Object%20Reference) (OtherBodyIndex :type Integer) (bFromSweep :type Boolean) (SweepResult :type Hit%20Result%20Structure%20%28by%20ref%29))
  (bind _asbp_comp_camera_guide_anchor (Utilities|Casting|CastToBP_CompCameraGuideAnchor OtherComp))
  (Utilities|Set|Add (Variables|Default|GetfocusAnchors) (Utilities|ResolveSoftReference _asbp_comp_camera_guide_anchor)))

(event OnComponentEndOverlap(Box)
  (params (OverlappedComponent :type Primitive%20Component%20Object%20Reference) (OtherActor :type Actor%20Object%20Reference) (OtherComp :type Primitive%20Component%20Object%20Reference) (OtherBodyIndex :type Integer))
  (bind _asbp_comp_camera_guide_anchor (Utilities|Casting|CastToBP_CompCameraGuideAnchor OtherComp))
  (Utilities|Set|Remove (Variables|Default|GetfocusAnchors) (Utilities|ResolveSoftReference _asbp_comp_camera_guide_anchor)))

(event EventBeginPlay
  (bind _box (Variables|Default|GetBox))
  (bind (_outcomponents _returnvalue) (Class|KismetSystemLibrary|ComponentOverlapComponents _box (Transformation|GetWorldTransform _box) (Utilities|Array|MakeArray "ObjectTypeQuery7") "/Game/blueprint/BP_CompCameraGuideAnchor.BP_CompCameraGuideAnchor_C"))
  (if _returnvalue
    (for _array_element _outcomponents
      (bind _asbp_comp_camera_guide_anchor (Utilities|Casting|CastToBP_CompCameraGuideAnchor _array_element))
      (Utilities|Set|Add (Variables|Default|GetfocusAnchors) (Utilities|ResolveSoftReference _asbp_comp_camera_guide_anchor)))))

(event Collision|EventActorBeginOverlap
  (params (OtherActor :type Actor%20Object%20Reference)))

(event EventTick
  (params (DeltaSeconds :type Float%20%28single-precision%29)))

(fn ConstructionScript
  (bind _box (Variables|Default|GetBox))
  (if (Variables|Default|GetInitEmpty)
    (Variables|/Script/Engine.PrimitiveComponent|SetbGenerateOverlapEvents _box false)
    (Components|Box|SetBoxExtent _box "0, 0, 0" false)))

(fn GetFocusLocation
  (bind _totleweight (LocalVariables|GettotleWeight))
  (bind _outlocation (LocalVariables|GetoutLocation))
  (bind _result (Utilities|Set|ToArray (Variables|Default|GetfocusAnchors)))
  (for _array_element _result
    (Utilities|FlowControl|Sequence
      (:then_0
        (|SetBy-RefVar _outlocation (+ _outlocation (* (Transformation|GetWorldLocation (Utilities|ResolveSoftReference _array_element)) (Variables|/Script/my2Dtry.CameraGuideAnchorComp|GetfocusWeight (Utilities|ResolveSoftReference _array_element))))))
      (:then_1
        (|SetBy-RefVar _totleweight (+ _totleweight (Variables|/Script/my2Dtry.CameraGuideAnchorComp|GetfocusWeight (Utilities|ResolveSoftReference _array_element)))))))
  (return (/ (LocalVariables|GetoutLocation) (LocalVariables|GettotleWeight))))

(fn AddGuideRefrence
  (params (anchor :type BP%20Comp%20Camera%20Guide%20Anchor%20Object%20Reference))
  (Utilities|Set|Add (Variables|Default|GetfocusAnchors) (Utilities|ResolveSoftReference anchor)))