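; BP_CompCameraActor drives its player-controlled owner's camera from the BP_CameraGuideVolumes it overlaps.
; On BeginPlay it seeds a volume stack with a spawned empty default volume, then, for player-controlled owners, spawns a BP_RectCamera as the view target.
; Overlap events push or remove volumes and pass the top entry to the camera, so leaving a volume falls back to the latest remaining one.
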(event Custom|OnComponentEndOverlap_Event
  (params (OverlappedComponent :type Primitive%20Component%20Object%20Reference) (OtherActor :type Actor%20Object%20Reference) (OtherComp :type Primitive%20Component%20Object%20Reference) (OtherBodyIndex :type Integer))
  (bind _volumestack (Variables|Default|GetvolumeStack))
  ;[1 1 1] Comment
  (bind _asbp_camera_guide_volume (Utilities|Casting|CastToBP_CameraGuideVolume OtherActor))
  (Utilities|Array|RemoveItem (Variables|Default|GetvolumeStack) _asbp_camera_guide_volume)
  (Default|ChangeVolume (Variables|Default|GetplayerCamera) (Utilities|Array|Get(acopy) _volumestack (Utilities|Array|LastIndex _volumestack))))

(event Custom|OnComponentBeginOverlap_Event
  (params (OverlappedComponent :type Primitive%20Component%20Object%20Reference) (OtherActor :type Actor%20Object%20Reference) (OtherComp :type Primitive%20Component%20Object%20Reference) (OtherBodyIndex :type Integer) (bFromSweep :type Boolean) (SweepResult :type Hit%20Result%20Structure%20%28by%20ref%29))
  (bind _volumestack (Variables|Default|GetvolumeStack))
  ;[1 1 1] camera volume
  (bind _asbp_camera_guide_volume (Utilities|Casting|CastToBP_CameraGuideVolume OtherActor))
  (Utilities|Array|AddUnique (Variables|Default|GetvolumeStack) _asbp_camera_guide_volume)
  (Default|ChangeVolume (Variables|Default|GetplayerCamera) (Utilities|Array|Get(acopy) _volumestack (Utilities|Array|LastIndex _volumestack))))

(event EventBeginPlay
  (bind _returnvalue (Components|GetOwner))
  ;[1 1 1] Create Rect Camera
  (|CallParentFunction)
  (Utilities|FlowControl|Sequence
    (:then_0
      (EventDispatchers|BindEventtoOnComponentBeginOverlap (delegate Custom|OnComponentBeginOverlap_Event))
      (EventDispatchers|BindEventtoOnComponentEndOverlap (delegate Custom|OnComponentEndOverlap_Event))
      (bind _returnvalue_2 (Game|SpawnActorfromClass "/Game/blueprint/BP_CameraGuideVolume.BP_CameraGuideVolume_C" (Math|Conversions|ToTransform(Vector) (Math|Vector|VectorZero)) "Undefined" 0 true 0))
      (Utilities|Array|Add (Variables|Default|GetvolumeStack) _returnvalue_2)
      (Default|AddGuideRefrence _returnvalue_2 self))
    (:then_1
      (if (Pawn|IsPlayerControlled (Variables|/Script/Engine.Actor|GetInstigator _returnvalue))
        (bind _returnvalue_3 (Game|SpawnActorfromClass "/Game/blueprint/BP_RectCamera.BP_RectCamera_C" (Transformation|GetActorTransform _returnvalue) "Undefined" 0 0))
        (bind _output_get (Variables|Default|SetplayerCamera _returnvalue_3))
        (bind _asplayer_controller (Utilities|Casting|CastToPlayerController (Pawn|GetController (Variables|/Script/Engine.Actor|GetInstigator (Components|GetOwner)))))
        (Game|Player|SetViewTargetwithBlend _asplayer_controller _output_get 0.0 "VTBlend_Linear" 0.0 false)
        (Default|ChangeVolume _output_get (Utilities|Array|Get(acopy) (Variables|Default|GetvolumeStack)))))))

(event EventTick
  (params (DeltaSeconds :type Float%20%28single-precision%29))
  (|CallParentFunction DeltaSeconds) ; This node is disabled and will not be called.\nDrag off pins to build functionality.
)