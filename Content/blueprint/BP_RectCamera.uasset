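; Camera rig that follows the focus location of a BP_CameraGuideVolume using nested rectangles in the XZ plane.
; BeginPlay finds the starting volume by box overlap, and ChangeVolume blends the actor to a new volume's focus with a timeline-driven lerp.
; Each tick, the difference between the actor-anchored inner rect and spring-arm-anchored outer rect offsets the spring arm.
; Debug boxes visualize both rects in construction and every tick.
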(event Custom|Change%20Volume
  (params (NewParam :type BP%20Camera%20Guide%20Volume%20Object%20Reference))
  (Variables|Default|SetcameraGuideVolumeIn NewParam)
  (Variables|Default|SetchangingVolume true)
  (Variables|Default|SettempBeginChangeLocation (Transformation|GetActorLocation))
  (bind _newtrack_0 (Timeline|changVolume PlayFromStart)
    (:Update
      (Transformation|SetActorLocation (Math|Vector|Lerp(Vector) (Math|Vector|Lerp(Vector) (Variables|Default|GettempBeginChangeLocation) (Transformation|GetActorLocation) _newtrack_0) (Default|GetFocusLocation (Variables|Default|GetcameraGuideVolumeIn)) _newtrack_0) false false))
    (:Finished
      (Variables|Default|SetchangingVolume false))))

(event EventBeginPlay
  (bind _box (Variables|Default|GetBox))
  (bind (_outactors _returnvalue) (Collision|ComponentOverlapActors _box (Transformation|GetWorldTransform _box) (Utilities|Array|MakeArray "ObjectTypeQuery7") 0))
  (if _returnvalue
    (bind _asbp_camera_guide_volume (Utilities|Casting|CastToBP_CameraGuideVolume (Utilities|Array|Get(acopy) _outactors)))
    (Variables|Default|SetcameraGuideVolumeIn _asbp_camera_guide_volume)))

(event Collision|EventActorBeginOverlap
  (params (OtherActor :type Actor%20Object%20Reference)))

(event EventTick
  (params (DeltaSeconds :type Float%20%28single-precision%29))
  (Utilities|FlowControl|Sequence
    (:then_0
      (if (Utilities|IsValid (Variables|Default|GetcameraGuideVolumeIn))
        (if (not (Variables|Default|GetchangingVolume))
          (Transformation|SetActorLocation (Default|GetFocusLocation (Variables|Default|GetcameraGuideVolumeIn)) false false))))
    (:then_1
      (Utilities|DebugDraw))
    (:then_2
      (Variables|Default|Setdelta (CallFunction|MyRectSub (CallFunction|MyRectAddVector (Variables|Default|GetinnerRect) (Transformation|GetActorLocation)) (CallFunction|MyRectAddVector (Variables|Default|GetoutterRect) (Transformation|GetWorldLocation (Variables|Default|GetSpringArm))))))
    (:then_3
      (if (not (Math|Vector|VectorIsZero (Variables|Default|Getdelta)))
        (Transformation|AddWorldOffset (Variables|Default|GetSpringArm) (Variables|Default|Getdelta) false false)))))

(fn ConstructionScript
  (Utilities|FlowControl|Sequence
    (:then_0
      (Utilities|DebugDraw))
    (:then_1
      (Transformation|SetWorldLocation (Variables|Default|GetSpringArm) (Transformation|GetActorLocation) false false))))