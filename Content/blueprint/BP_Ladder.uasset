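; BP_Ladder is a Paper2D ladder actor that builds itself in the construction script from the LocationTop vector, with no active event logic.
; The script zeroes LocationTop's Y, then sizes and raises the Box component to span the height, using X as its half-width.
; It then stacks collision-free BlockSprite components every BlockStep up to that height, leaving the Box as the ladder's volume.
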(event EventBeginPlay)

(event Collision|EventActorBeginOverlap
  (params (OtherActor :type Actor%20Object%20Reference)))

(event EventTick
  (params (DeltaSeconds :type Float%20%28single-precision%29)))

(fn ConstructionScript
  (Utilities|FlowControl|Sequence
    (:then_0
      (Variables|Default|SetLocationTop (Math|Vector|MakeVector (.x (Variables|Default|GetLocationTop)) 0.0 (.z (Variables|Default|GetLocationTop))))
      (Components|Box|SetBoxExtent (Variables|Default|GetBox) (Math|Vector|MakeVector (.x (Variables|Default|GetLocationTop)) 1e+01 (/ (.z (Variables|Default|GetLocationTop)) 2.0)) true)
      (Transformation|AddLocalOffset (Variables|Default|GetBox) (Math|Vector|MakeVector 0.0 0.0 (/ (.z (Variables|Default|GetLocationTop)) 2.0)) false false))
    (:then_1
      (for _index (range 0 (Math|Float|Truncate (/ (.z (Variables|Default|GetLocationTop)) (Variables|Default|GetBlockStep))))
        (bind _returnvalue (AddComponent|AddPaperSpriteComponent false))
        (Rendering|Components|Sprite|SetSprite _returnvalue (Variables|Default|GetblockSprite))
        (Transformation|AddLocalOffset _returnvalue (Math|Vector|MakeVector 0.0 0.0 (* _index (Variables|Default|GetBlockStep))) false false)
        (Collision|SetCollisionEnabled _returnvalue "NoCollision")))))